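; Basement_Slock is an interactable basement prop that, when used, swaps itself for Basement_Slock_2 and reveals a diary page.
; A Box overlap with BP_FirstPersonCharacter enables input and opens a Gate, and leaving disables input and closes it.
; Pressing Interact while the Gate is open spawns Basement_Slock_2 at the StaticMesh transform and DiaryPage1_4 at the Diary transform, then destroys this actor.
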(event `InputAction|Interact`
  (params (Key :type "Key Structure"))
  (:`Pressed`
    (if true
      (`/Engine/EditorBlueprintResources/StandardMacros.Gate` true :!label _label
        (:`Exit`
          (`|SpawnActorFromClass` "/Game/ZimingFile/Assets/Ziming/Blueprint/Basement_Slock_2.Basement_Slock_2_C" (`SceneComponent.K2_GetComponentToWorld` (`self.StaticMesh`)) "Undefined" "OverrideRootScale" null null)
          (`|SpawnActorFromClass` "/Game/Diary/DiaryPage1_4.DiaryPage1_4_C" (`SceneComponent.K2_GetComponentToWorld` (`self.Diary`)) "Undefined" "OverrideRootScale" null null)
          (`self.K2_DestroyActor`))))))

(event `self.Box.OnComponentBeginOverlap`
  (params (OverlappedComponent :type "PrimitiveComponent Object Reference") (OtherActor :type "Actor Object Reference") (OtherComp :type "PrimitiveComponent Object Reference") (OtherBodyIndex :type Integer) (bFromSweep :type Boolean) (SweepResult :type "HitResult Structure (by ref)"))
  (cast `/Game/FirstPerson/Blueprints/BP_FirstPersonCharacter` OtherActor)
  (`self.EnableInput` (`GameplayStatics.GetPlayerController` 0))
  (goto _label :!via `Open`))

(event `self.Box.OnComponentEndOverlap`
  (params (OverlappedComponent :type "PrimitiveComponent Object Reference") (OtherActor :type "Actor Object Reference") (OtherComp :type "PrimitiveComponent Object Reference") (OtherBodyIndex :type Integer))
  (cast `/Game/FirstPerson/Blueprints/BP_FirstPersonCharacter` OtherActor)
  (`self.DisableInput` (`GameplayStatics.GetPlayerController` 0))
  (goto _label :!via `Close`))

(fn `UserConstructionScript`)